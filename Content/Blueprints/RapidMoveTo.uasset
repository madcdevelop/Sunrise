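; Behavior tree task that moves a Follower_AI_CON's pawn to the actor in the TargetToFollow blackboard key.
; On execute, it casts and caches the controller only if none is stored, then starts AI MoveTo with a small acceptance radius.
; A successful move finishes the task as failed.
; A failed move, failed cast or already cached controller never calls FinishExecute.
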(event `self.ReceiveExecute`
  (params (OwnerActor :type "Actor Object Reference"))
  (if (not (!= (`self.AI_CON_REF`) null))
    (bind _asfollower_ai_con (cast `/Game/Blueprints/Follower_AI_CON` OwnerActor))
    (set `self.AI_CON_REF` _asfollower_ai_con)
    (`|AIMoveTo` (`Controller.K2_GetPawn` (`self.AI_CON_REF`)) (0.0 0.0 0.0) (`BTFunctionLibrary.GetBlackboardValueAsActor` (`self.TargetToFollow`)) 50.0
      (:`OnSuccess`
        (`self.FinishExecute` false)))))