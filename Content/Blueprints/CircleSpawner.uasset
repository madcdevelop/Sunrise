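; CircleSpawner is an actor that spawns a set number of CharacterClass actors in an evenly spaced ring when play begins.
; On BeginPlay it loops over SpawnCount, rotating a Radius-long vector by CurrentAngle plus an equal yaw step to place each spawn around the Capsule's world location.
; Spawns keep zero world rotation and always spawn regardless of collision.
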(event `self.ReceiveBeginPlay`
  (for _index (range 1 (+ (`self.SpawnCount`) 1))
    (`|SpawnActorFromClass` (`self.CharacterClass`) (`KismetMathLibrary.MakeTransform` (+ (`SceneComponent.K2_GetComponentLocation` (`self.Capsule`)) (`KismetMathLibrary.GreaterGreater_VectorRotator` (`KismetMathLibrary.MakeVector` (`self.Radius`)) (`KismetMathLibrary.MakeRotator` 0.0 0.0 (+ (`self.CurrentAngle`) (* (`KismetMathLibrary.Conv_IntToDouble` _index) (/ 360.0 (`KismetMathLibrary.Conv_IntToDouble` (`self.SpawnCount`))))))))) "AlwaysSpawn" "OverrideRootScale" null null)))

(fn `UserConstructionScript`)