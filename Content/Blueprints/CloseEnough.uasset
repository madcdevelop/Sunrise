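; CloseEnough is a Behavior Tree decorator for follower AI that tests the distance to its follow target.
; It casts the owner to Follower_AI_CON and measures from the controlled pawn to the actor in the TargetToFollow blackboard key.
; Despite its name, the condition returns true when that distance is at or beyond AcceptableDistance, meaning the follower is not yet close.
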(fn `PerformConditionCheck`
  (params (OwnerActor :type "Actor Object Reference"))
  (returns (ReturnValue :type Boolean))
  (bind _asfollower_ai_con (cast `/Game/Blueprints/Follower_AI_CON` OwnerActor))
  (set `self.AI_CON_REF` _asfollower_ai_con)
  (return (>= (`KismetMathLibrary.VSize` (- (`Actor.K2_GetActorLocation` (`BTFunctionLibrary.GetBlackboardValueAsActor` (`self.TargetToFollow`))) (`Actor.K2_GetActorLocation` (`Controller.K2_GetPawn` (`self.AI_CON_REF`))))) (`self.AcceptableDistance`))))