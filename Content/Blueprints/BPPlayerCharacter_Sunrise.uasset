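; Player character Blueprint that equips a sword and a shield when play begins.
; BeginPlay calls a reusable AttachWeapon function once for the right hand socket and once for the left.
; AttachWeapon spawns the given class at the mesh socket's world transform, ignoring collisions, then snaps it to that socket.
; Tick and the construction script are empty.
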(event `self.ReceiveBeginPlay`
  ;[1 1 1] Character equip
  (`self.AttachWeapon` (`self.RightHandSocket`) (`self.WeaponSword`))
  (`self.AttachWeapon` (`self.LeftHandSocket`) (`self.ItemShield`)))

(event `self.ReceiveTick`
  (params (DeltaSeconds :type "Float (single-precision)")))

(fn `AttachWeapon`
  (params (SocketName :type Name) (`Class Reference` :type "Actor Class Reference"))
  ;[1 1 1] Attach Weapon to Character Socket
  (bind _returnvalue (`|SpawnActorFromClass` `Class Reference` (`SceneComponent.GetSocketTransform` (`self.Mesh`) SocketName "RTS_World") "AlwaysSpawn" "OverrideRootScale" null null))
  (`self.K2_AttachToComponent` _returnvalue (`self.Mesh`) SocketName "SnapToTarget" "SnapToTarget" "SnapToTarget" true))

(fn `UserConstructionScript`)